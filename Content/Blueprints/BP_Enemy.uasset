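; BP_Enemy is an enemy that flies in a straight line and explodes on contact.
; On BeginPlay it finds BP_Player and picks a fixed direction: 30% of the time toward the player, otherwise straight down, aligning its Z axis to it.
; Tick moves it by Speed along that direction without sweep.
; Any Box overlap destroys both the other actor and itself, with explosion sound and particles.
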(event `self.ReceiveBeginPlay`
  (bind _returnvalue (`GameplayStatics.GetActorOfClass` "/Game/Blueprints/BP_Player.BP_Player_C"))
  (set `self.Target` _returnvalue)
  (`self.FindTargetDirection`))

(event `self.ReceiveTick`
  (params (DeltaSeconds :type "Float (single-precision)"))
  (`self.K2_SetActorLocation` (+ (`self.K2_GetActorLocation`) (* DeltaSeconds (* (`self.Speed`) (`self.Direction`))))))

(event `self.Box.OnComponentBeginOverlap`
  (params (OverlappedComponent :type "PrimitiveComponent Object Reference") (OtherActor :type "Actor Object Reference") (OtherComp :type "PrimitiveComponent Object Reference") (OtherBodyIndex :type Integer) (bFromSweep :type Boolean) (SweepResult :type "HitResult Structure (by ref)"))
  (`self.K2_DestroyActor` OtherActor)
  (`GameplayStatics.PlaySound2D` "/Game/ShootingAssets/Audios/자료실_2장_Explosion.자료실_2장_Explosion" 1.0 1.0 0.0 null null)
  (`GameplayStatics.SpawnEmitterAtLocation` "/Game/StarterContent/Particles/P_Explosion.P_Explosion" (`self.K2_GetActorLocation`))
  (`self.K2_DestroyActor`))

(fn `FindTargetDirection`
  ;[1 1 1] 타겟 존재 검사
  (`/Engine/EditorBlueprintResources/StandardMacros.IsValid` (`self.Target`)
    (:`Is Valid`
      (if (<= (`KismetMathLibrary.RandomIntegerInRange` 1 100) 30)
        ;[1 1 1] 타겟 방향 찾기
        (bind _output_get (set `self.Direction` (`KismetMathLibrary.Normal` (- (`self.K2_GetActorLocation` (`self.Target`)) (`self.K2_GetActorLocation`)))))
        (else
          (set `self.Direction` (0.0 0.0 -1.0) :!label _label))))
    (:`Is Not Valid`
      (goto _label)))
  (`self.K2_SetActorRotation` (`KismetMathLibrary.MakeRotFromZX` _output_get (`self.GetActorForwardVector`))))

(fn `UserConstructionScript`)