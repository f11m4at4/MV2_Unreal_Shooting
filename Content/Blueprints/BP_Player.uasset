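; BP_Player is the player actor of a simple shooter that flies in the Y-Z plane and fires bullets.
; Each Tick it builds a direction from the horizontal and vertical input getters, scales it by Speed and delta time, and sets the new location without sweep.
; The Fire action spawns a BP_Bullet at the actor's location and plays a blaster sound.
; An unrelated Print205 function repeatedly prints a name string in a loop.
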(event `self.ReceiveBeginPlay`)

(event `self.ReceiveTick`
  (params (DeltaSeconds :type "Float (single-precision)"))
  ;[1 1 1] 이동하고 싶다.
  (set `self.Direction` (`KismetMathLibrary.MakeVector` 0.0 (`self.GetInputAxisValue`) (`self.GetInputAxisValue`)))
  (set `self.P0` (`self.K2_GetActorLocation`))
  (set `self.vt` (* (* DeltaSeconds (`self.Speed`)) (`self.Direction`)))
  (bind _output_get (set `self.P` (+ (`self.P0`) (`self.vt`))))
  (`self.K2_SetActorLocation` _output_get))

(event `InputAction|Fire`
  (params (Key :type "Key Structure"))
  (:`Pressed`
    (`|SpawnActorFromClass` "/Game/Blueprints/BP_Bullet.BP_Bullet_C" (`KismetMathLibrary.MakeTransform` (`self.K2_GetActorLocation`)) "Undefined" "MultiplyWithRoot" null null)
    (`GameplayStatics.PlaySound2D` "/Game/ShootingAssets/Audios/자료실_2장_star-wars-blaster.자료실_2장_star-wars-blaster" 1.0 1.0 0.0 null null)))

(fn `Print205`
  (for _ (range 101)
    (`KismetSystemLibrary.PrintString` "이영호")))

(fn `UserConstructionScript`)